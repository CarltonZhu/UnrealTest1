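; BP_Player is the playable character Blueprint, handling core movement through Enhanced Input.
; BeginPlay adds the IMC_CarltonsContext mapping context and puts the Carltons_HUD widget on the viewport.
; Input actions drive movement along the actor's forward and right vectors, mouse look with inverted pitch input, and jumping.
; Sprint and crouch are hold-style, with sprint raising max walk speed until release.
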(event Input|EnhancedActionEvents|EnhancedInputActionWASD_Movement
  (params (ActionValue :type Vector%202D%20Structure) (ElapsedSeconds :type Float%20%28double-precision%29) (TriggeredSeconds :type Float%20%28double-precision%29) (InputAction :type Input%20Action%20Object%20Reference :default "/Game/Core/Input/WASD_Movement.WASD_Movement"))
  ;[1 1 1] CORE MOVEMENT
  (:Triggered
    (Pawn|Input|AddMovementInput (Transformation|GetActorForwardVector) (.x ActionValue) false)
    (Pawn|Input|AddMovementInput (Transformation|GetActorRightVector) (.y ActionValue) false)))

(event Input|EnhancedActionEvents|EnhancedInputActionMouse_Movement
  (params (ActionValue :type Vector%202D%20Structure) (ElapsedSeconds :type Float%20%28double-precision%29) (TriggeredSeconds :type Float%20%28double-precision%29) (InputAction :type Input%20Action%20Object%20Reference :default "/Game/Core/Input/Mouse_Movement.Mouse_Movement"))
  ;[1 1 1] CORE MOVEMENT
  (:Triggered
    (Pawn|Input|AddControllerYawInput (.x ActionValue))
    (Pawn|Input|AddControllerPitchInput (* (.y ActionValue) -1.0))))

(event Input|EnhancedActionEvents|EnhancedInputActionJump
  (params (ActionValue :type Boolean) (ElapsedSeconds :type Float%20%28double-precision%29) (TriggeredSeconds :type Float%20%28double-precision%29) (InputAction :type Input%20Action%20Object%20Reference :default "/Game/Core/Input/Jump.Jump"))
  ;[1 1 1] CORE MOVEMENT
  (:Started
    (Character|Jump)))

(event Input|EnhancedActionEvents|EnhancedInputActionShiftRun
  (params (ActionValue :type Boolean) (ElapsedSeconds :type Float%20%28double-precision%29) (TriggeredSeconds :type Float%20%28double-precision%29) (InputAction :type Input%20Action%20Object%20Reference :default "/Game/Core/Input/ShiftRun.ShiftRun"))
  (bind _charactermovement (Variables|Character|GetCharacterMovement))
  ;[1 1 1] CORE MOVEMENT
  (:Started
    (Variables|/Script/Engine.CharacterMovementComponent|SetMaxWalkSpeed _charactermovement 1.2e+03))
  (:Completed
    (Variables|/Script/Engine.CharacterMovementComponent|SetMaxWalkSpeed _charactermovement 6e+02)))

(event Input|EnhancedActionEvents|EnhancedInputActionCrouch
  (params (ActionValue :type Boolean) (ElapsedSeconds :type Float%20%28double-precision%29) (TriggeredSeconds :type Float%20%28double-precision%29) (InputAction :type Input%20Action%20Object%20Reference :default "/Game/Core/Input/Crouch.Crouch"))
  ;[1 1 1] CORE MOVEMENT
  (:Started
    (Character|Crouch))
  (:Completed
    (Character|UnCrouch)))

(event EventBeginPlay
  ;[1 1 1] CORE MOVEMENT
  (Input|AddMappingContext (PlayerController|LocalPlayerSubsystems|GetEnhancedInputLocalPlayerSubsystem (Game|GetPlayerController 0)) "/Game/Core/Input/IMC_CarltonsContext.IMC_CarltonsContext" 0 "(bIgnoreAllPressedKeysUntilRelease=True,bForceImmediately=False,bNotifyUserSettings=False)")
  (bind _returnvalue (UserInterface|CreateWidget "/Game/UI/Carltons_HUD.Carltons_HUD_C"))
  (UserInterface|Viewport|AddtoViewport _returnvalue 0))

(fn ConstructionScript)